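; BP_RisasStudent is a Paper2D student character that laughs in response to an event from the player's BP_MainCharacter.
; On BeginPlay it sets its starting flipbook and binds to the player's AmigoRisas event, which passes along a key.
; Q, W, E and R each select a laugh stage with its own flipbook and 2D sound.
; After a per-stage delay, longer at each stage, it switches to the idle flipbook.
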(event `self.ReceiveBeginPlay`
  (`PaperFlipbookComponent.SetFlipbook` (`self.PaperFlipbook`) (`self.FlipBookStudent`))
  (bind _asbp_main_character (cast `/Game/Character/BP_MainCharacter` (`GameplayStatics.GetPlayerPawn` 0)))
  (add `/Game/Character/BP_MainCharacter.AmigoRisas` _asbp_main_character (delegate `RisaySonido`)))

(event `RisaySonido`
  (params (KeyPressed :type String))
  (`self.Play sound base on Key` KeyPressed))

(event `Play sound base on Key`
  (params (KeyPreseed :type String))
  (switch `string` KeyPreseed
    (:`Q`
      (`PaperFlipbookComponent.SetFlipbook` (`self.PaperFlipbook`) "/Game/Sprites/Characters/Friend/amigo_risa_1/amigo_risa_1.amigo_risa_1")
      (`GameplayStatics.PlaySound2D` "/Game/Music/Friend/3__Risa_stage_1.3__Risa_stage_1" 1.0 1.0 0.0 null null)
      (`KismetSystemLibrary.Delay` 1.0)
      (`PaperFlipbookComponent.SetFlipbook` (`self.PaperFlipbook`) "/Game/Sprites/Characters/Friend/Amigo_idle/amigo_idle.amigo_idle"))
    (:`W`
      (`PaperFlipbookComponent.SetFlipbook` (`self.PaperFlipbook`) "/Game/Sprites/Characters/Friend/aigo_risa_2/amigo_risa_2.amigo_risa_2")
      (`GameplayStatics.PlaySound2D` "/Game/Music/Friend/4__RIsa_Stage_2.4__RIsa_Stage_2" 1.0 1.0 0.0 null null)
      (`KismetSystemLibrary.Delay` 1.5)
      (`PaperFlipbookComponent.SetFlipbook` (`self.PaperFlipbook`) "/Game/Sprites/Characters/Friend/Amigo_idle/amigo_idle.amigo_idle"))
    (:`E`
      (`PaperFlipbookComponent.SetFlipbook` (`self.PaperFlipbook`) "/Game/Sprites/Characters/Friend/Amigo_risa_3/Amigo_risa_3.Amigo_risa_3")
      (`GameplayStatics.PlaySound2D` "/Game/Music/Friend/5__RIsa_Stage_3.5__RIsa_Stage_3" 1.0 1.0 0.0 null null)
      (`KismetSystemLibrary.Delay` 2.0)
      (`PaperFlipbookComponent.SetFlipbook` (`self.PaperFlipbook`) "/Game/Sprites/Characters/Friend/Amigo_idle/amigo_idle.amigo_idle"))
    (:`R`
      (`PaperFlipbookComponent.SetFlipbook` (`self.PaperFlipbook`) "/Game/Sprites/Characters/Friend/amigo_risa_4/amigo_risa_4.amigo_risa_4")
      (`GameplayStatics.PlaySound2D` "/Game/Music/Friend/6__RIsa_stage_4_Laughter.6__RIsa_stage_4_Laughter" 1.0 1.0 0.0 null null)
      (`KismetSystemLibrary.Delay` 4.0)
      (`PaperFlipbookComponent.SetFlipbook` (`self.PaperFlipbook`) "/Game/Sprites/Characters/Friend/Amigo_idle/amigo_idle.amigo_idle"))))

(fn `UserConstructionScript`)