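; Teacher catch effect actor that plays a "caught" flipbook and freezes the player when the Teacher's Catch event fires.
; On BeginPlay it binds to Catch, then disables player input, plays the non-looping Teacher_Caught flipbook after a short delay and sets a Teacher blackboard bool.
; When playback finishes, it clears the flipbook, resets the bool and restores input.
; The finish handler is assigned on every catch, after playback starts.
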(event `self.ReceiveBeginPlay`
  (add `/Game/AI/BP_Teacher.Catch` (`self.Teacher`) (delegate `CustomEvent`)))

(event `CustomEvent`
  (bind _returnvalue (`GameplayStatics.GetPlayerController` 0))
  (`self.DisableInput` (`Controller.K2_GetPawn` _returnvalue) _returnvalue)
  (`PaperFlipbookComponent.SetFlipbook` (`self.PaperFlipbook`) "/Game/Sprites/Characters/Teacher/Caught/Teacher_Caught.Teacher_Caught")
  (`PaperFlipbookComponent.SetLooping` (`self.PaperFlipbook`) false)
  (`KismetSystemLibrary.Delay` 0.2)
  (`PaperFlipbookComponent.PlayFromStart` (`self.PaperFlipbook`))
  (`BlackboardComponent.SetValueAsBool` (`AIBlueprintHelperLibrary.GetBlackboard` (`self.Teacher`)) (`self.Key`) true)
  (add `PaperFlipbookComponent.OnFinishedPlaying` (`self.PaperFlipbook`) (delegate `OnFinishedPlaying_Event`)))

(event `OnFinishedPlaying_Event`
  (bind _returnvalue (`GameplayStatics.GetPlayerController` 0))
  (`PaperFlipbookComponent.SetFlipbook` (`self.PaperFlipbook`) null)
  (`BlackboardComponent.SetValueAsBool` (`AIBlueprintHelperLibrary.GetBlackboard` (`self.Teacher`)) (`self.Key`) false)
  (`self.EnableInput` (`Controller.K2_GetPawn` _returnvalue) _returnvalue))

(fn `UserConstructionScript`)