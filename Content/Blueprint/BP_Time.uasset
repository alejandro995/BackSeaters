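; BP_Time is a countdown Blueprint that ends the game in a loss when time runs out.
; BeginPlay sets the remaining time to 90 seconds and starts a looping one-second timer that calls DecreaseTime by name.
; Each tick prints a debug string and decrements the counter; once it reaches zero, it sets Win to false on the GS_BSS Game Instance and opens LVL_End.
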(event `self.ReceiveBeginPlay`
  (set `self.Time Remaining` 90.0)
  (`KismetSystemLibrary.K2_SetTimer` null "DecreaseTime" 1.0 true))

(event `DecreaseTime`
  (`KismetSystemLibrary.PrintText` "time")
  (if (<= (`self.Time Remaining`) 0.0)
    (bind _asgs_bss (cast `/Game/GameMode/GS_BSS` (`GameplayStatics.GetGameInstance`)))
    (set `/Game/GameMode/GS_BSS.Win` false _asgs_bss)
    (`GameplayStatics.OpenLevel` "LVL_End")
    (else
      (set `self.Time Remaining` (- (`self.Time Remaining`) 1.0)))))

(fn `UserConstructionScript`)