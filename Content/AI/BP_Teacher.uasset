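; Teacher AI that uses PawnSensing to catch the main character when it is seen with a matching gameplay tag.
; A catch calls CallCatch, plays two audio components in sequence, then pauses the player's sounds and flipbook after a brief delay.
; A TeacherCatching flag blocks repeat catches until the delays finish.
; BeginPlay fills origin and destination index arrays, likely for a route, which this graph never reads.
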(event `self.ReceiveBeginPlay`
  (set `self.LoopIndex` 0)
  (set `self.OriginIndexArray` (`|MakeArray` 1 0 3 6 7 8 5 4 1 2 0 0 0))
  (set `self.DestinationIndexArray` (`|MakeArray` 0 3 6 7 4 5 8 7 4 3 6 3 0 1 4 5 8 7 8 5 4 3 0 1 4 5 2 5 2 5 8)))

(event `self.PawnSensing.OnSeePawn`
  (params (Pawn :type "Pawn Object Reference"))
  (if (not (`self.TeacherCatching`))
    (bind _asbp_main_character (cast `/Game/Character/BP_MainCharacter` Pawn))
    (set `self.Player` _asbp_main_character)
    (if (`BlueprintGameplayTagLibrary.HasTag` (`/Game/Character/BP_MainCharacter.Tag` _asbp_main_character) (struct :`TagName` "Cast") true)
      (set `self.TeacherCatching` true)
      (`self.Catch`)
      (bind _returnvalue (`AddComponent|NODE_AddAudioComponent-0`))
      (add `AudioComponent.OnAudioFinished` _returnvalue (delegate `OnAudioFinished_Event`))
      (`KismetSystemLibrary.Delay` 0.3)
      (`self.StopPlayer`)
      (`KismetSystemLibrary.Delay` 6.5)
      (set `self.TeacherCatching` false))))

(event `OnAudioFinished_Event`
  (`KismetSystemLibrary.Delay` 0.25)
  (`AddComponent|NODE_AddAudioComponent-1`))

(event `StopPlayer`
  (bind _player (`self.Player`))
  (`/Game/Character/BP_MainCharacter.PauseSounds` _player)
  (`PaperFlipbookComponent.Stop` (`/Game/Character/BP_MainCharacter.PaperFlipbook` _player)))

(fn `UserConstructionScript`)