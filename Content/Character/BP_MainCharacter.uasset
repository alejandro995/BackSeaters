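; Main character Blueprint with four meme-themed abilities on Q, W, E and R, R being the ultimate.
; Each press broadcasts KeyPressed with its stats, plays a sound, then calls AmigoRisas and returns to idle after timed delays.
; A Cast gameplay tag blocks overlapping casts, while per-key booleans gate cooldowns.
; Q, W and E re-arm after their delays; R's flag clears after casting and is never restored here.
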(event `Key|Q`
  (params (Key :type "Key Structure"))
  ;[1 1 1] Q
  (:`Pressed`
    (if (and (not (`BlueprintGameplayTagLibrary.HasTag` (`self.Tag`) (struct :`TagName` "Cast"))) (`self.QColdown`))
      (`self.KeyPressed` "Q" 5 1.5 1.5 1.0)
      (`self.Add Tag`)
      (`GameplayStatics.PlaySound2D` "/Game/Music/Powers/9_Q_1_5s.9_Q_1_5s" 1.0 1.0 0.0 null null)
      (set `self.QColdown` false)
      (`KismetSystemLibrary.Delay` 1.5)
      (`self.AmigoRisas` "Q")
      (`self.Idle`)
      (`self.RemoveTag`)
      (`KismetSystemLibrary.Delay` 1.5)
      (set `self.QColdown` true))))

(event `Key|W`
  (params (Key :type "Key Structure"))
  ;[1 1 1] W
  (:`Pressed`
    (if (and (not (`BlueprintGameplayTagLibrary.HasTag` (`self.Tag`) (struct :`TagName` "Cast"))) (`self.WColdown`))
      (`self.KeyPressed` "w" 10 2.0 3.0 3.0)
      (`self.Add Tag`)
      (`GameplayStatics.PlaySound2D` "/Game/Music/Powers/10_W_buscando_meme_.10_W_buscando_meme_" 1.0 1.0 0.0 null null)
      (set `self.WColdown` false)
      (`KismetSystemLibrary.Delay` 2.5)
      (`self.RemoveTag`)
      (`KismetSystemLibrary.Delay` 0.5)
      (`self.AmigoRisas` "W")
      (`self.Idle`)
      (`KismetSystemLibrary.Delay` 2.0)
      (set `self.WColdown` true))))

(event `Key|E`
  (params (Key :type "Key Structure"))
  ;[1 1 1] E
  (:`Pressed`
    (if (and (not (`BlueprintGameplayTagLibrary.HasTag` (`self.Tag`) (struct :`TagName` "Cast"))) (`self.EColdown`))
      (`self.KeyPressed` "E" 20 3.0 5.0 5.0)
      (`self.Add Tag`)
      (`GameplayStatics.PlaySound2D` "/Game/Music/Powers/11__Gigachad_1.11__Gigachad_1" 1.0 1.0 0.0 null null)
      (set `self.EColdown` false)
      (`KismetSystemLibrary.Delay` 4.5)
      (`self.RemoveTag`)
      (`KismetSystemLibrary.Delay` 0.5)
      (`self.AmigoRisas` "E")
      (`self.Idle`)
      (`KismetSystemLibrary.Delay` 3.0)
      (set `self.EColdown` true))))

(event `Key|R`
  (params (Key :type "Key Structure"))
  ;[1 1 1] R
  (:`Pressed`
    (if (and (not (`BlueprintGameplayTagLibrary.HasTag` (`self.Tag`) (struct :`TagName` "Cast"))) (`self.RColdown`))
      (`self.KeyPressed` "R" 50 0.0 7.0 0.0 10)
      (`self.Add Tag`)
      (`GameplayStatics.PlaySound2D` "/Game/Music/Powers/12__R_Ult_Sound_7s.12__R_Ult_Sound_7s" 1.0 1.0 0.0 null null)
      (`KismetSystemLibrary.Delay` 6.5)
      (`self.RemoveTag`)
      (`KismetSystemLibrary.Delay` 0.5)
      (`self.AmigoRisas` "R")
      (`self.Idle`)
      (set `self.RColdown` false))))

(event `Idle`
  (`self.KeyPressed` "idle"))

(event `Add Tag`
  (`BlueprintGameplayTagLibrary.AddGameplayTag` (`self.Tag`) (struct :`TagName` "Cast")))

(event `RemoveTag`
  (`BlueprintGameplayTagLibrary.RemoveGameplayTag` (`self.Tag`) (struct :`TagName` "Cast")))

(fn `UserConstructionScript`)